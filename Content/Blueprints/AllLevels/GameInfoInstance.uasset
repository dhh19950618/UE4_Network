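; GameInfoInstance is a game instance-style hub for front-end menus and multiplayer sessions.
; SaveGameCheck opens the main menu if a player settings save exists, otherwise the options menu; most widgets are created once and cached.
; It creates, joins and destroys sessions behind a loading screen for create and join, opening Lobby as a listen server.
; Errors only print, and the network and travel error-to-string functions are empty stubs.
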(event Custom|ShowMainMenu
  (bind _returnvalue (Game|GetPlayerController 0))
  ;[1 1 1] 显示主菜单和鼠标
  (Utilities|IsValid (Variables|Widgets|GetMainMenuWB)
    (:Is%20Valid
      _)
    (:Is%20Not%20Valid
      (bind _returnvalue_2 (UserInterface|CreateWidget "/Game/UI/MainMenu/MainMenu.MainMenu_C" _returnvalue))
      (Variables|Widgets|SetMainMenuWB _returnvalue_2)))
  (UserInterface|Viewport|AddtoViewport (Variables|Widgets|GetMainMenuWB) 0)
  (Variables|/Script/Engine.PlayerController|SetbShowMouseCursor _returnvalue true))

(event Custom|ShowLoadingScreen
  ;[1 1 1] 显示加载界面
  (Utilities|IsValid (Variables|Default|GetLoadingScreenWB)
    (:Is%20Valid
      _)
    (:Is%20Not%20Valid
      (bind _returnvalue (UserInterface|CreateWidget "/Game/UI/AllLevels/LoadingScreen.LoadingScreen_C" (Game|GetPlayerController 0)))
      (Variables|Default|SetLoadingScreenWB _returnvalue)))
  (UserInterface|Viewport|AddtoViewport (Variables|Default|GetLoadingScreenWB) 0))

(event Custom|SaveGameCheck
  ;[1 1 1] 检查个人信息存储
  (bind _returnvalue (SaveGame|DoesSaveGameExist (Variables|Default|GetPlayerSettingsSave)))
  (if _returnvalue
    (CallFunction|ShowMainMenu)
    (Variables|Default|SetisCreateSaveFiles true)
    (else
      (CallFunction|ShowOptionsMenu)
      (Variables|/Script/Engine.PlayerController|SetbShowMouseCursor (Game|GetPlayerController 0) true))))

(event Custom|ShowServeMenu
  ;[1 1 1] 创建服务器菜单 - 每次触发都创建
  (bind _returnvalue (UserInterface|CreateWidget "/Game/UI/MainMenu/ServeMenu.ServeMenu_C" (Game|GetPlayerController 0)))
  (UserInterface|Viewport|AddtoViewport _returnvalue 0))

(event Custom|JoinServe
  (params (SessionToJoin :type Blueprint%20Session%20Result%20Structure))
  ;[1 1 1] 加入房间
  (CallFunction|ShowLoadingScreen)
  (|JoinSession (Game|GetPlayerController 0) SessionToJoin
    (:OnFailure
      (Utilities|DisplayErrorMessage "Failed to join session,Try again"))))

(event Custom|ShowOptionsMenu
  ;[1 1 1] 显示选项菜单
  (Utilities|IsValid (Variables|Widgets|GetOptionsMenuWB)
    (:Is%20Valid
      _)
    (:Is%20Not%20Valid
      (bind _returnvalue (UserInterface|CreateWidget "/Game/UI/MainMenu/OptionsMenu.OptionsMenu_C" (Game|GetPlayerController 0)))
      (Variables|Widgets|SetOptionsMenuWB _returnvalue)))
  (UserInterface|Viewport|AddtoViewport (Variables|Widgets|GetOptionsMenuWB) 0)
  (if (not (Variables|Default|GetisCreateSaveFiles))
    (Variables|/Game/UI/MainMenu/OptionsMenu.OptionsMenu_C|SetVisibleHelloText (Variables|Widgets|GetOptionsMenuWB) "Visible")))

(event Custom|DestroySessionCaller
  (params (PlayerController :type Player%20Controller%20Object%20Reference))
  ;[1 1 1] 关闭房间
  (|DestroySession PlayerController))

(event Custom|ShowHostMenu
  ;[1 1 1] 客户端主菜单
  (Utilities|IsValid (Variables|Widgets|GetHostMenuWB)
    (:Is%20Valid
      _)
    (:Is%20Not%20Valid
      (bind _returnvalue (UserInterface|CreateWidget "/Game/UI/MainMenu/HostMenu.HostMenu_C" (Game|GetPlayerController 0)))
      (Variables|Widgets|SetHostMenuWB _returnvalue)))
  (UserInterface|Viewport|AddtoViewport (Variables|Widgets|GetHostMenuWB) 0))

(event Custom|LaunchLobby
  (params (NumOfPlayers :type Integer) (EnableLan :type Boolean) (SeverName :type Text))
  ;[1 1 1] 加载大厅&客户端设置
  (Variables|ServerSettings|SetMaxPlayers NumOfPlayers)
  (Variables|ServerSettings|SetServeName SeverName)
  (CallFunction|ShowLoadingScreen)
  (|Session (Game|GetPlayerController 0) (Variables|ServerSettings|GetMaxPlayers) EnableLan
    (:OnSuccess
      (Game|OpenLevel(byName) "Lobby" true "listen"))
    (:OnFailure
      (Utilities|DisplayErrorMessage "Failed to Create Session,Please try again"))))

(event EventHandleNetworkError
  (params (FailureType :type ENetworkFailure%20Enum :default "NetDriverAlreadyExists") (bIsServer :type Boolean))
  ;[1 1 1] 处理网络错误
  (if bIsServer
    _
    (else
      _))
  (Utilities|DisplayErrorMessage (CallFunction|NetErrortoString FailureType)))

(event EventHandleTravelError
  (params (FailureType :type ETravelFailure%20Enum :default "NoLevel"))
  ;[1 1 1] 处理传输错误
  (Utilities|DisplayErrorMessage (CallFunction|TravelErrortoString FailureType)))

(fn NetErrortoString
  (params (FailureType :type ENetworkFailure%20Enum :default "NetDriverAlreadyExists"))
  (return ""))

(fn TravelErrortoString
  (params (FailureType :type ETravelFailure%20Enum :default "NoLevel"))
  (return ""))