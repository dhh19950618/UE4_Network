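; LobbyGM is the lobby game mode that registers joining players and keeps every lobby screen in sync.
; PostLogin reads server settings from GameInfoInstance, sets up the LobbyPC menu, then spawns a default 0_Base pawn at a random PlayerStart.
; EveryoneUpdate shares player settings, counts and available characters with all controllers, setting CanWeStart from whether players still use 0_Base.
; Kick, character swap and game launch events are empty stubs.
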(event Custom|SwapCharacter
  (params (PlayerController :type Player%20Controller%20Object%20Reference) (CharacterClass :type Character%20Class%20Reference) (ChangeStatus :type Boolean)))

(event Custom|LaunchTheGame)

(event Custom|AddToKickList)

(event Custom|CannotStartGame
  ;[1 1 1] 更新所有连接玩家的信息
  (Utilities|Array|ForEachLoopwithBreak (Variables|ServerSettings|GetConnectedPlayers)) ; enters at Break
)

(event Custom|EveryoneUpdate
  (bind _allplayercontrollers (Variables|ServerSettings|GetAllPlayerControllers))
  ;[1 1 1] 更新所有连接玩家的信息
  (bind _output_get (Variables|ServerSettings|SetCurrentPlayers (Utilities|Array|Length (Variables|ServerSettings|GetAllPlayerControllers))))
  (if (> _output_get 0)
    (Utilities|Array|Clear (Variables|ServerSettings|GetConnectedPlayers))
    (for _array_element _allplayercontrollers
      (bind _aslobby_pc (Utilities|Casting|CastToLobbyPC _array_element))
      (Utilities|Array|Add (Variables|ServerSettings|GetConnectedPlayers) (Variables|/Game/Blueprints/Lobby/LobbyPC.LobbyPC_C|GetPlaySettings _aslobby_pc))
      (Default|UpdateNumberOfPlayers _aslobby_pc (Variables|ServerSettings|GetCurrentPlayers) (Variables|ServerSettings|GetMaxPlayers)))
    (for _array_element_2 _allplayercontrollers
      (bind _aslobby_pc_2 (Utilities|Casting|CastToLobbyPC _array_element_2))
      (Default|AddPlayerInfo _aslobby_pc_2 (Variables|ServerSettings|GetConnectedPlayers))
      (Default|UpdateAvalibleCharacters _aslobby_pc_2 (Variables|ServerSettings|GetisAvalibleCharacters))
      (CallFunction|AddtoKickList))
    (bind _array_element_3 (Utilities|Array|ForEachLoopwithBreak (Variables|ServerSettings|GetConnectedPlayers))
      (:LoopBody
        (if (== (.MyPlayerCharacter (Utilities|Struct|BreakPlayerInfo _array_element_3)) "/Game/Blueprints/Characters/0_Base.0_Base_C")
          (Variables|ServerSettings|SetcanWeStart false)
          (CallFunction|CannotStartGame)
          (else
            (Variables|ServerSettings|SetcanWeStart true)))))))

(event Custom|RespawnPlayer
  (params (PlayerController :type Player%20Controller%20Object%20Reference))
  (bind _returnvalue (Pawn|GetControlledPawn PlayerController))
  (bind _spawnpoints (Variables|ServerSettings|GetSpawnPoints))
  ;[1 1 1] 玩家角色初始化 - 重生
  (Utilities|IsValid _returnvalue
    (:Is%20Valid
      (Actor|DestroyActor _returnvalue))
    (:Is%20Not%20Valid
      _))
  (bind _returnvalue_2 (Game|SpawnActorfromClass "/Game/Blueprints/Characters/0_Base.0_Base_C" (Transformation|GetActorTransform (Utilities|Array|Get(acopy) _spawnpoints (Math|Random|RandomIntegerinRange 0 (- (Utilities|Array|Length _spawnpoints) 1)))) "Undefined" 0 0))
  (Pawn|Possess PlayerController _returnvalue_2)
  (CallFunction|EveryoneUpdate))

(event EventPostLogin
  (params (NewPlayer :type Player%20Controller%20Object%20Reference))
  ;[1 1 1] 玩家加入后的初始化设置
  (Networking|SwitchHasAuthority
    (:Authority
      (Utilities|Array|Add (Variables|ServerSettings|GetAllPlayerControllers) NewPlayer)
      (bind _outactors (Actor|GetAllActorsOfClass "/Script/Engine.PlayerStart"))
      (Variables|ServerSettings|SetSpawnPoints _outactors)
      (bind _asgame_info_instance (Utilities|Casting|CastToGameInfoInstance (Game|GetGameInstance)))
      (Variables|ServerSettings|SetServeName (Variables|/Game/Blueprints/AllLevels/GameInfoInstance.GameInfoInstance_C|GetServeName _asgame_info_instance))
      (Variables|ServerSettings|SetMaxPlayers (Variables|/Game/Blueprints/AllLevels/GameInfoInstance.GameInfoInstance_C|GetMaxPlayers _asgame_info_instance))
      (bind _aslobby_pc (Utilities|Casting|CastToLobbyPC NewPlayer))
      (Default|InitialSetup _aslobby_pc)
      (Default|SetupLobbyMenu _aslobby_pc (Variables|ServerSettings|GetServeName))
      (Default|UpdateLobbySettings _aslobby_pc (Variables|ServerSettings|GetGM_MapImage) (Variables|ServerSettings|GetGM_MapName) (Variables|ServerSettings|GetGM_MapTime))
      (CallFunction|RespawnPlayer NewPlayer))))

(fn ConstructionScript)